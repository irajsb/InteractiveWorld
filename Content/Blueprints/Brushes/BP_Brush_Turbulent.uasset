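; Brush that stamps a turbulence material onto a drawing board's render target canvas along its movement path.
; On BeginPlay it creates a dynamic instance of M_TurbulentBrush.
; Each DrawonRT call, gated on the last draw succeeding, scales Strength by distance moved per draw step and Height relative to InteractDistance.
; It then draws at a position interpolated between previous and current transforms, converted from world to canvas space.
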(event EventBeginPlay
  (|CallParentFunction)
  (bind _returnvalue (Rendering|Material|CreateDynamicMaterialInstance "/InteractiveWorld/Materials/BrushMaterials/M_TurbulentBrush.M_TurbulentBrush" "None" "None" :!class /Script/Engine.KismetMaterialLibrary))
  (Variables|Default|SetTurbulentMaterial _returnvalue))

(event EventTick
  (params (DeltaSeconds :type Float%20%28single-precision%29))
  (|CallParentFunction DeltaSeconds) ; 此节点被禁用，将不会被调用。\n从引脚连出引线来编译功能。
)

(event EventDrawonRT
  (params (DrawingBoard :type World%20Drawing%20Board%20Object%20Reference) (CanvasDrawOn :type Canvas%20Object%20Reference) (CanvasSize :type Vector%202D%20Structure) (InterpolateRate :type Float%20%28single-precision%29) (DrawTimes :type Integer))
  (bind _size (Variables|Default|GetSize))
  (bind _turbulentmaterial (Variables|Default|GetTurbulentMaterial))
  (bind _currentt (Variables|Default|GetCurrentT))
  (bind _previoust (Variables|Default|GetPreviousT))
  (bind _returnvalue (Math|Vector|Lerp(Vector) (.location _previoust) (.location _currentt) InterpolateRate))
  (bind _returnvalue_2 (Math|Conversions|ToVector2D(Vector) _returnvalue))
  (bind (_outscreenposition _outscreensize _outscreenrotation) (Class|WorldDrawingBoard|WorldtoCanvasBrush DrawingBoard _returnvalue_2 _size 0.0))
  (if (Class|InteractBrush|GetLastDrawSucceed)
    (Rendering|Material|SetScalarParameterValue _turbulentmaterial "Strength" (* (/ (Math|Vector|VectorLength (- (.location _currentt) (.location _previoust))) (Math|Conversions|ToFloat(Integer) DrawTimes)) (Variables|Turbulent|GetStrength)) :!class /Script/Engine.MaterialInstanceDynamic)
    (Rendering|Material|SetScalarParameterValue _turbulentmaterial "Height" (/ (Variables|Default|GetHeight) (Variables|Default|GetInteractDistance)) :!class /Script/Engine.MaterialInstanceDynamic)
    (Canvas|DrawMaterial :self CanvasDrawOn :RenderMaterial _turbulentmaterial :ScreenPosition _outscreenposition :ScreenSize _outscreensize :CoordinateSize "(X=1.000000,Y=1.000000)" :Rotation _outscreenrotation :PivotPoint "(X=0.500000,Y=0.500000)")))